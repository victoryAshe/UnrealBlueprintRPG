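; Bear enemy that chases the player, deals damage through a toggled attack collision, and dissolves on death.
; A tick-driven state machine mirrors its state to the AI blackboard and sets walk speed per state.
; PawnSensing starts chases, while distance or the player's state returns it to Locomotion.
; BPHPController receives damage and signals death, and timelines animate material hit flash and dissolve before destruction.
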(event `UpdateState`
  (params (`New State` :type "/Game/Bluprints/Monster/EBearState Enum" :default "NewEnumerator0"))
  (bind _charactermovement (`self.CharacterMovement`))
  ; 몬스터 상태 변경 이벤트.
  (if (`|EnumInequality` (`self.State_BP`) "NewEnumerator3")
    (bind _output_get (set `self.State_BP` `New State`))
    (`BlackboardComponent.SetValueAsEnum` (`AIController.Blackboard` (`AIBlueprintHelperLibrary.GetAIController` self)) (`self.StateKey`) _output_get)
    (switch `/Game/Bluprints/Monster/EBearState` (`self.State_BP`)
      (:`NewEnumerator0`
        (set `CharacterMovementComponent.MaxWalkSpeed` 200.0 _charactermovement))
      (:`NewEnumerator1`
        (set `CharacterMovementComponent.MaxWalkSpeed` 300.0 _charactermovement))
      (:`NewEnumerator2`
        (set `CharacterMovementComponent.MaxWalkSpeed` 0.0 _charactermovement :!label _label))
      (:`NewEnumerator3`
        (goto _label)))))

(event `self.ReceiveBeginPlay`
  ;[0 0.466 0.1036 0.5] 죽음 Event에 바인딩.
  (add `/Game/Bluprints/Components/BP_HPController.OnDeadEvent` (`self.BP_HPController`) (delegate `RecievedOnDead`))
  ;; 시작할 때 Attack Collision 끄기.
  (`PrimitiveComponent.SetCollisionEnabled` (`self.AttackCollision`) "NoCollision"))

(event `RecievedOnDead`
  (bind _mesh (`self.Mesh`))
  ;[0 0.466 0.1036 0.5] 죽음 Event에 바인딩.
  (set `self.State_BP` "NewEnumerator3")
  (`PrimitiveComponent.SetCollisionEnabled` (`self.CapsuleComponent`) "NoCollision")
  (`KismetSystemLibrary.Delay` 2.0)
  (bind (_direction _dissolve _hitvalue) (`Timeline|DeathEffect`)
    (:`Update`
      (`MeshComponent.SetScalarParameterValueOnMaterials` _mesh "Dissolve" _dissolve)
      (`MeshComponent.SetScalarParameterValueOnMaterials` _mesh "HitValue" _hitvalue))
    (:`Finished`
      (`self.K2_DestroyActor`))))

(event `self.ReceiveActorBeginOverlap`
  (params (OtherActor :type "Actor Object Reference"))
  ; PlayerWeapon Hit 처리.
  (if (`self.ActorHasTag` OtherActor "PlayerWeapon")
    (bind (_direction _hitvalue) (`Timeline|HitEffect` :!via `PlayFromStart`)
      (:`Update`
        (`MeshComponent.SetScalarParameterValueOnMaterials` (`self.Mesh`) "HitValue" _hitvalue)))))

(event `self.ReceiveAnyDamage`
  (params (Damage :type "Float (single-precision)") (DamageType :type "DamageType Object Reference") (InstigatedBy :type "Controller Object Reference") (DamageCauser :type "Actor Object Reference"))
  ; HP 처리.
  (`/Game/Bluprints/Components/BP_HPController.ReceiveDamage` (`self.BP_HPController`) Damage))

(event `self.PawnSensing.OnSeePawn`
  (params (Pawn :type "Pawn Object Reference"))
  ; Player감지.
  (if (`|EnumEquality` (`self.State_BP`) "NewEnumerator0")
    (if (`self.ActorHasTag` Pawn "Player")
      (`BlackboardComponent.SetValueAsObject` (`AIController.Blackboard` (`AIBlueprintHelperLibrary.GetAIController` self)) (`self.TargetPlayerKey`) Pawn)
      (bind _asbp_character (cast `/Game/Bluprints/Character/BP_Character` Pawn))
      (if (not (`|EnumEquality` (`/Game/Bluprints/Character/BP_Character.State_BP` _asbp_character) "NewEnumerator2"))
        (`self.UpdateState` "NewEnumerator1")))))

(event `self.ReceiveTick`
  (params (DeltaSeconds :type "Float (single-precision)"))
  ; Tick마다 동작하는 간단한 FSM.
  (switch `/Game/Bluprints/Monster/EBearState` (`self.State_BP`)
    (:`NewEnumerator0`
      (`self.OnLocomotion`))
    (:`NewEnumerator1`
      (`self.OnChase`))
    (:`NewEnumerator2`
      (`self.OnAttack`))
    (:`NewEnumerator3`
      (`self.OnDead`))))

(event `OnAttackCheckStart`
  ; 공격 판정 시작/종료
  (`PrimitiveComponent.SetCollisionEnabled` (`self.AttackCollision`) "QueryOnly"))

(event `OnAttackCheckEnd`
  ; 공격 판정 시작/종료
  (`PrimitiveComponent.SetCollisionEnabled` (`self.AttackCollision`) "NoCollision"))

(event `self.AttackCollision.OnComponentBeginOverlap`
  (params (OverlappedComponent :type "PrimitiveComponent Object Reference") (OtherActor :type "Actor Object Reference") (OtherComp :type "PrimitiveComponent Object Reference") (OtherBodyIndex :type Integer) (bFromSweep :type Boolean) (SweepResult :type "HitResult Structure (by ref)"))
  ; Player에 Damage 전달
  (`GameplayStatics.ApplyDamage` OtherActor (`self.Damage`) (`self.GetController`) self))

(fn `OnAttack`
  (bind _asbp_character (cast `/Game/Bluprints/Character/BP_Character` (`BlackboardComponent.GetValueAsObject` (`AIController.Blackboard` (`AIBlueprintHelperLibrary.GetAIController` self)) (`self.TargetPlayerKey`))))
  (if (`|EnumEquality` (`/Game/Bluprints/Character/BP_Character.State_BP` _asbp_character) "NewEnumerator2")
    (`self.UpdateState` "NewEnumerator0")))

(fn `OnChase`
  (bind _asactor (cast `Actor` (`BlackboardComponent.GetValueAsObject` (`AIController.Blackboard` (`AIBlueprintHelperLibrary.GetAIController` self)) (`self.TargetPlayerKey`))))
  (if (> (`KismetMathLibrary.Vector_Distance` (`self.K2_GetActorLocation` _asactor) (`self.K2_GetActorLocation`)) (`PawnSensingComponent.SightRadius` (`self.PawnSensing`)))
    (`self.UpdateState` "NewEnumerator0")))

(fn `OnDead`)

(fn `OnLocomotion`)

(fn `UserConstructionScript`)