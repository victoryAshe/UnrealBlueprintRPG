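; BP_HPController is a health component that tracks its owner's HealthPower and reacts to incoming damage.
; ReceiveDamage subtracts positive damage while health is above zero.
; When health drops to zero or below, it calls OnDeadEvent, and the guard on current health keeps later hits from triggering it again.
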(event `ReceiveDamage`
  (params (Damage :type "Float (double-precision)"))
  (if (> (`self.HealthPower`) 0.0)
    (if (> Damage 0.0)
      (bind _output_get (set `self.HealthPower` (- (`self.HealthPower`) Damage)))
      (if (<= _output_get 0.0)
        (`self.OnDeadEvent`)))))