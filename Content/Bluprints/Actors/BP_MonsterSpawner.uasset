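; BP_MonsterSpawner is an actor that spawns a monster of MonsterClass at a random actor from SpawnPoints.
; StartSpawning sets a three-second timer that calls SpawnMonster.
; A valid spawn increments SpawnCount without rescheduling, while a failed spawn calls StartSpawning to retry.
; The TargetSpawnCount comparison and GameMode cast are unconnected, so no spawn limit is enforced.
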(event `StartSpawning`
  ;[0.422 0 0 0.5] 몬스터 생성.
  (`KismetSystemLibrary.K2_SetTimerDelegate` (delegate `SpawnMonster`) 3.0))

(event `SpawnMonster`
  ;[0.422 0 0 0.5] 몬스터 생성.
  (bind _returnvalue (`|SpawnActorFromClass` (`self.MonsterClass`) (`self.GetTransform` (`KismetArrayLibrary.Array_Random` (`self.SpawnPoints`))) "Undefined" "MultiplyWithRoot" null null))
  (`/Engine/EditorBlueprintResources/StandardMacros.IsValid` _returnvalue
    (:`Is Valid`
      (bind _result (`/Engine/EditorBlueprintResources/StandardMacros.IncrementInt` (`self.SpawnCount`))))
    (:`Is Not Valid`
      (`self.StartSpawning`))))

(fn `UserConstructionScript`)