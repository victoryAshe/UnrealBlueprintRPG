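; Player controller that sets up gameplay input and the main HUD, and relays game-mode events to it.
; On BeginPlay it switches to game-only input, adds the IMC_Game Enhanced Input context, creates WBP_MainUI and binds to BP_GameMode's kill count, stage clear and game over events.
; Kill updates go straight to the widget, while stage clear and game over also switch to UI-only input and show the cursor.
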(event `self.ReceiveBeginPlay`
  (`WidgetBlueprintLibrary.SetInputMode_GameOnly` self)
  (set `self.bShowMouseCursor` false)
  (`EnhancedInputSubsystemInterface.AddMappingContext` (subsystem `EnhancedInputLocalPlayerSubsystem`) "/Game/Bluprints/Input/IMC_Game.IMC_Game" 0 (struct))
  (bind _returnvalue (`|CreateWidget` "/Game/UI/WBP_MainUI.WBP_MainUI_C"))
  (bind _output_get (set `self.MainUI` _returnvalue))
  (`UserWidget.AddToViewport` _output_get 0)
  (bind _asbp_game_mode (cast `/Game/Bluprints/Character/BP_GameMode` (`GameplayStatics.GetGameMode`)))
  (add `/Game/Bluprints/Character/BP_GameMode.OnKillCountUpdated` _asbp_game_mode (delegate `OnKillCountUpdated`))
  (add `/Game/Bluprints/Character/BP_GameMode.OnStageClear` _asbp_game_mode (delegate `OnStageClear`))
  (add `/Game/Bluprints/Character/BP_GameMode.OnGameOver` _asbp_game_mode (delegate `OnGameOver`)))

(event `OnKillCountUpdated`
  (params (CurrentKills :type Integer) (TargetKills :type Integer))
  (`/Game/UI/WBP_MainUI.OnKillCountUpdated` (`self.MainUI`) CurrentKills TargetKills))

(event `OnStageClear`
  (bind _mainui (`self.MainUI`))
  (`/Game/UI/WBP_MainUI.StageClear` _mainui)
  (`WidgetBlueprintLibrary.SetInputMode_UIOnlyEx` self _mainui)
  (set `self.bShowMouseCursor` true))

(event `OnGameOver`
  (bind _mainui (`self.MainUI`))
  (`/Game/UI/WBP_MainUI.GameOver` _mainui)
  (`WidgetBlueprintLibrary.SetInputMode_UIOnlyEx` self _mainui)
  (set `self.bShowMouseCursor` true))

(fn `UserConstructionScript`)