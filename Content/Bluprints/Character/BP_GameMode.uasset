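; Game mode Blueprint that tracks kill progress and signals the stage clear and game over states.
; MonsterKilled increments the kill count, broadcasts it with the target, and broadcasts stage clear when the two are equal.
; PlayerDied broadcasts game over, GameStart forwards to a GameStart call, and RestartGame reopens the main level.
; Event dispatchers carry these state changes to listeners, with no Tick logic.
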(event `GameStart`
  ;[0.08653 0.502 0 0.5] 게임 시작 이벤트.
  (`self.GameStart`))

(event `MonsterKilled`
  (bind _result (`/Engine/EditorBlueprintResources/StandardMacros.IncrementInt` (`self.CurrentKills`))
    (:`  `
      (`self.OnKillCountUpdated` _result (`self.TargetKills`))
      ; 스테이지 클리어 조건 확인 및 이벤트 발생
      (if (== (`self.CurrentKills`) (`self.TargetKills`))
        (`self.OnStageClear`)))))

(event `PlayerDied`
  ; Game Over
  (`self.OnGameOver`))

(event `RestartGame`
  ; 게임 재시작
  (`GameplayStatics.OpenLevelBySoftObjectPtr` "/Game/Maps/MainLevel.MainLevel"))

(fn `UserConstructionScript`)