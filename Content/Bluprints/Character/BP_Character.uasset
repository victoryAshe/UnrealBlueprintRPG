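; Player character Blueprint handling movement, camera look, jumping, combo melee attacks, weapon pickup, damage and death.
; A Locomotion/Battle/Dead state gates input, with attack presses queuing the next combo from the current montage section.
; A collected weapon attaches to a hand-placement socket and receives hit-check windows through event dispatchers.
; HPController processes damage and drives the HP bar and death, while hits trigger camera shake and a material flash.
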(event `ReceiveOnHPChanged`
  (params (HealthPower :type "Float (double-precision)") (MaxHealthPower :type "Float (double-precision)"))
  ; 시작 시: 죽음 Event에 Binding. (Subscription)
  (bind _aswbp_hpbar (cast `/Game/UI/WBP_HPBar` (`WidgetComponent.GetUserWidgetObject` (`self.HPBar`))))
  (`/Game/UI/WBP_HPBar.UpdateHpPercent` _aswbp_hpbar (/ HealthPower MaxHealthPower)))

(event `self.ReceiveBeginPlay`
  ; 시작 시: 죽음 Event에 Binding. (Subscription)
  (add `/Game/Bluprints/Components/BP_HPController.OnDeadEvent` (`self.HPController`) (delegate `Receive OnDeadEvent`))
  (add `/Game/Bluprints/Components/BP_HPController.OnHPChanged` (`self.HPController`) (delegate `ReceiveOnHPChanged`)))

(event `Receive OnDeadEvent`
  ; 시작 시: 죽음 Event에 Binding. (Subscription)
  (`PrimitiveComponent.SetCollisionEnabled` (`self.CapsuleComponent`) "NoCollision")
  (set `self.State_BP` "NewEnumerator2"))

(event `EnhancedInput|/Game/Bluprints/Input/Actions/IA_Move`
  (params (ActionValue :type "Vector2D Structure") (ElapsedSeconds :type "Float (double-precision)") (TriggeredSeconds :type "Float (double-precision)") (InputAction :type "InputAction Object Reference" :default "/Game/Bluprints/Input/Actions/IA_Move.IA_Move"))
  (bind (_returnvalue_roll _returnvalue_pitch _returnvalue_yaw) (`KismetMathLibrary.BreakRotator` (`self.GetControlRotation`)))
  ;[0.04463 0.265 0 0.5] 이동
  (:`Triggered`
    (switch `/Game/Bluprints/Character/EPlayerState` (`self.State_BP`)
      (:`NewEnumerator0`
        (`self.AddMovementInput` (`KismetMathLibrary.GetRightVector` (`self.GetControlRotation`)) ActionValue_X)
        (`self.AddMovementInput` (`KismetMathLibrary.GetForwardVector` (`KismetMathLibrary.MakeRotator` 0.0 0.0 _returnvalue_yaw)) ActionValue_Y)))))

(event `EnhancedInput|/Game/Bluprints/Input/Actions/IA_View`
  (params (ActionValue :type "Vector2D Structure") (ElapsedSeconds :type "Float (double-precision)") (TriggeredSeconds :type "Float (double-precision)") (InputAction :type "InputAction Object Reference" :default "/Game/Bluprints/Input/Actions/IA_View.IA_View"))
  ;[0.665 0.4528 0 0.5] 카메라 회전
  (:`Triggered`
    (`self.AddControllerYawInput` ActionValue_X) ; Controller에 Yaw 회전 추가
    (`self.AddControllerPitchInput` ActionValue_Y) ; Controller에 Pitch 회전 추가
  ))

(event `EnhancedInput|/Game/Bluprints/Input/Actions/IA_Attack`
  (params (ActionValue :type Boolean) (ElapsedSeconds :type "Float (double-precision)") (TriggeredSeconds :type "Float (double-precision)") (InputAction :type "InputAction Object Reference" :default "/Game/Bluprints/Input/Actions/IA_Attack.IA_Attack"))
  ;[0.42 0 0 0.5] 공격
  (:`Started`
    (if (`self.HasWeapon`)
      ;; 일반 상태인지 확인
      (switch `/Game/Bluprints/Character/EPlayerState` (`self.State_BP`)
        (:`NewEnumerator0`
          (set `self.State_BP` "NewEnumerator1")
          (`self.PlayAnimMontage` "/Game/Bluprints/Character/AM_Attack.AM_Attack"))
        (:`NewEnumerator1`
          (switch `name` (`AnimInstance.Montage_GetCurrentSection` (`SkeletalMeshComponent.GetAnimInstance` (`self.Mesh`)) "/Game/Bluprints/Character/AM_Attack.AM_Attack")
            (:`Attack1`
              (set `self.NextCombo` "Attack2"))
            (:`Attack2`
              (set `self.NextCombo` "Attack3"))
            (:`Attack3`
              (set `self.NextCombo` "Attack4"))))))))

(event `AttackEnd`
  ;[0.42 0 0 0.5] 공격
  (set `self.State_BP` "NewEnumerator0"))

(event `OnWeaponCollected`
  (params (WeaponActor :type "/Game/Bluprints/Actors/BP_Weapon Object Reference"))
  ;[0 0.798 0.04515 0.5] 무기 습득 처리.
  (`self.SetOwner` WeaponActor self)
  (`self.K2_AttachToComponent` WeaponActor (`self.Mesh`) "WeaponPosition" "SnapToTarget" "SnapToTarget" "SnapToTarget" true)
  (set `self.WeaponActor` WeaponActor)
  (set `self.HasWeapon` true)
  ;[0.759 0 0 0.5] 공격 판정 시작 Event 함수 등록(Subscription) => Observer Pattern.
  (add `self.AttackCheckBeginEvent` (delegate `RaiseAttackCheckBegin`))
  ;[0 0.36 0.1518 0.5] 공격 판정 종료 Event에 함수 등록(Subscription)
  (add `self.AttackCheckEndEvent` (delegate `RaiseAttackCheckEnd`)))

(event `RaiseAttackCheckBegin`
  ;[0.759 0 0 0.5] 공격 판정 시작 Event 함수 등록(Subscription) => Observer Pattern.
  (`/Engine/EditorBlueprintResources/StandardMacros.IsValid` (`self.WeaponActor`)
    (:`Is Valid`
      (`/Game/Bluprints/Actors/BP_Weapon.OnAttackCheckBegin` (`self.WeaponActor`)))))

(event `RaiseAttackCheckEnd`
  ;[0 0.36 0.1518 0.5] 공격 판정 종료 Event에 함수 등록(Subscription)
  (`/Engine/EditorBlueprintResources/StandardMacros.IsValid` (`self.WeaponActor`)
    (:`Is Valid`
      (`/Game/Bluprints/Actors/BP_Weapon.OnAttackCheckEnd` (`self.WeaponActor`)))))

(event `OnAttackCheckBegin`
  ;[0.91 0 0 0.5] 공격 판정 시작
  (`self.AttackCheckBeginEvent`))

(event `OnAttackCheckEnd`
  ;[0 0.213 0.08899 0.5] 공격 판정 종료
  (`self.AttackCheckEndEvent`))

(event `self.ReceiveAnyDamage`
  (params (Damage :type "Float (single-precision)") (DamageType :type "DamageType Object Reference") (InstigatedBy :type "Controller Object Reference") (DamageCauser :type "Actor Object Reference"))
  ;[0.898 0 0 0.5] 체력 관리 Component에 Damage 전달.
  (`CameraShakeSourceComponent.Start` (`self.CameraShake`))
  (`/Game/Bluprints/Components/BP_HPController.ReceiveDamage` (`self.HPController`) Damage)
  ;;[0.638 0.5717 0 0.5] 피격 효과.
  (bind (_direction _hitvalue) (`Timeline|HitEffect` :!via `PlayFromStart`)
    (:`Update`
      (`MeshComponent.SetScalarParameterValueOnMaterials` (`self.Mesh`) "HitValue" _hitvalue))))

(event `EnhancedInput|/Game/Bluprints/Input/Actions/IA_Jump`
  (params (ActionValue :type Boolean) (ElapsedSeconds :type "Float (double-precision)") (TriggeredSeconds :type "Float (double-precision)") (InputAction :type "InputAction Object Reference" :default "/Game/Bluprints/Input/Actions/IA_Jump.IA_Jump"))
  (:`Started`
    (switch `/Game/Bluprints/Character/EPlayerState` (`self.State_BP`)
      (:`NewEnumerator0`
        (`self.Jump`)))))

(fn `UserConstructionScript`)